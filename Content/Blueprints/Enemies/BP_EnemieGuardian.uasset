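; Guardian enemy that tracks its movement state for directional animation and signals when the player enters or leaves its detection range.
; Tick derives Direction from velocity with X and Y swapped, sets IsMoving, and updates LastDirection only when both axes are non-zero.
; DetectionRange overlaps filter for the BP_MyCharacter capsule, then fire the player in-range and out-of-range event dispatchers.
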(event OnComponentBeginOverlap(DetectionRange)
  (params (OverlappedComponent :type Primitive%20Component%20Object%20Reference) (OtherActor :type Actor%20Object%20Reference) (OtherComp :type Primitive%20Component%20Object%20Reference) (OtherBodyIndex :type Integer) (bFromSweep :type Boolean) (SweepResult :type Hit%20Result%20Structure%20%28by%20ref%29))
  ;[1 1 1] Llamamos a los Delegados de "Jugador en Rango"
  (Utilities|Casting|CastToCapsuleComponent OtherComp)
  (Utilities|Casting|CastToBP_MyCharacter OtherActor)
  ;;[1 1 1] Llamamos al Event "Jugador en Rango"
  (Default|CallOnPlayerinRange))

(event OnComponentEndOverlap(DetectionRange)
  (params (OverlappedComponent :type Primitive%20Component%20Object%20Reference) (OtherActor :type Actor%20Object%20Reference) (OtherComp :type Primitive%20Component%20Object%20Reference) (OtherBodyIndex :type Integer))
  ;[1 1 1] Llamamos a los Delegados de "Jugador salió Rango"
  (Utilities|Casting|CastToCapsuleComponent OtherComp)
  (Utilities|Casting|CastToBP_MyCharacter OtherActor)
  ;;[1 1 1] Llamamos al Event "Jugador salió de Rango"
  (Default|CallOnPlayerOutOfRange))

(event EventBeginPlay)

(event Collision|EventActorBeginOverlap
  (params (OtherActor :type Actor%20Object%20Reference)))

(event EventTick
  (params (DeltaSeconds :type Float%20%28single-precision%29))
  (bind _charactermovement (Variables|Character|GetCharacterMovement))
  (bind _velocity (Variables|/Script/Engine.MovementComponent|GetVelocity _charactermovement))
  ;[0 0.9143 1] Detección de Dirección de Animacion en base a Movimiento
  ;;[0.05127 0.1144 0.2423] Actualizamos la Direccion de movimiento
  (bind _output_get (Variables|Default|SetDirection (Math|Vector2D|MakeVector2D (.y _velocity) (.x _velocity))))
  ;;[0.2918 0.000304 0.000304] Controlamos si el Flag de "EnMovimiento" esta Activo, o no
  (Variables|Default|SetIsMoving (or (!= (.x _output_get) 0.0) (!= (.y _output_get) 0.0)))
  ;;[0.2961 0 0] Con la ultima direccion distinta de 0, almacenamos la ultima direccion en que se movio el Enemigo
  (if (and (!= (.x _output_get) 0.0) (!= (.y _output_get) 0.0))
    (Variables|Default|SetLastDirection (Math|Vector2D|MakeVector2D (.x _output_get) (.y _output_get)))))

(fn ConstructionScript)