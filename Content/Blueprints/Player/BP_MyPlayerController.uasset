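; Player controller that creates the HUD, sets game-only input and routes player actions to BP_MyCharacter and BP_ECGameMode.
; Enhanced Input drives single-axis movement without diagonals, updating Direction and signaling movement start and stop, commented as enemy notifications.
; Interact starts or advances nearby NPC dialogue, locking movement until EnablePlayerActions; another input triggers Soul Light.
; Start/Pause calls ChangeLevel, which plays a HUD fade before opening MainMenu.
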(event Custom|EnablePlayerActions
  ;[1 0.3104 0.2806] Activamos Flag de Jugador en Dialogo
  (Variables|/Game/Blueprints/Player/BP_MyCharacter.BP_MyCharacter_C|SetInDialogue (Variables|Default|GetPlayerCharacter) false)
  ;[1 0.3104 0.2806] Desactivamos Flag de "Jugador puede moverse"
  (Variables|/Game/Blueprints/Player/BP_MyCharacter.BP_MyCharacter_C|SetCanMove (Variables|Default|GetPlayerCharacter) true))

(event Custom|ChangeLevel
  (params (NextLevelName :type Name))
  (bind _w_hud_reference (Variables|Default|GetW_HUD_Reference))
  ;[1 0 0.2078] Reproducimos Animacion de Fade In en el Widget
  (Components|Animation|PlayAnimation _w_hud_reference (Variables|/Game/UI/HUD/W_HUD.W_HUD_C|GetFadeIn _w_hud_reference) 0.0
    (:Finished
      ;[0.07619 0.1912 0.3005] Cuando la animacion termine, salimos al Menu Principal
      (Game|OpenLevel(byName) NextLevelName))))

(event Input|EnhancedActionEvents|EnhancedInputActionIA_Move
  (params (ActionValue :type Vector%202D%20Structure) (ElapsedSeconds :type Float%20%28double-precision%29) (TriggeredSeconds :type Float%20%28double-precision%29) (InputAction :type Input%20Action%20Object%20Reference :default "/Game/Blueprints/Player/Input/IA_Move.IA_Move"))
  (:Triggered
    ;[0.06447 0.4112 1] Evento de Inputs de Movimiento
    ;;[0.8438 0.1187 0.1453] Comprobamos si el Personaje puede moverse
    (if (Variables|/Game/Blueprints/Player/BP_MyCharacter.BP_MyCharacter_C|GetCanMove (Variables|Default|GetPlayerCharacter))
      (if (and (!= (.x ActionValue) 0.0) (== (.y ActionValue) 0.0))
        ;;[0.231 0.5298 0.7552] Notificamos a los Enemigos que "Jugador empezo a moverse"
        (Default|CallOnPlayerStartedMovement)
        ;;[0 0.3734 0.8958] Agregamos Inputs de movimiento al Perosnaje
        (Pawn|Input|AddMovementInput (Variables|Default|GetPlayerCharacter) (Transformation|GetActorRightVector (Variables|Default|GetPlayerCharacter)) (.x ActionValue) false)
        ;[1 1 1] Actualizamos la variable de Dirección del Player
        (Variables|/Game/Blueprints/Player/BP_MyCharacter.BP_MyCharacter_C|SetDirection (Variables|Default|GetPlayerCharacter) (Math|Vector2D|MakeVector2D (.x ActionValue) (.y ActionValue)) :!label _label)
        (elif (and (== (.x ActionValue) 0.0) (!= (.y ActionValue) 0.0))
          ;;[0.231 0.5298 0.7552] Notificamos a los Enemigos que "Jugador empezo a moverse"
          (Default|CallOnPlayerStartedMovement)
          ;;[0 0.3734 0.8958] Agregamos Inputs de movimiento al Perosnaje
          (Pawn|Input|AddMovementInput (Variables|Default|GetPlayerCharacter) (Transformation|GetActorForwardVector (Variables|Default|GetPlayerCharacter)) (.y ActionValue) false)
          (goto _label)
          (else
            ;;[0.1248 0.2874 0.4072] Notificamos a los Enemigos que  "Jugador dejó de moverse"
            (Default|CallOnPlayerStoppedMovement))))))
  (:Started
    ;[0.231 0.5298 0.7552] Notificamos a los Enemigos que "Jugador empezo a moverse"
    (Default|CallOnPlayerStartedMovement))
  (:Completed
    ;[0.1248 0.2874 0.4072] Notificamos a los Enemigos que  "Jugador dejó de moverse"
    (Default|CallOnPlayerStoppedMovement)))

(event EventBeginPlay
  ;[1 0 0.2078] Creamos un Widget del HUD, lo almacenamos, y agregamos al Viewport
  (bind _returnvalue (UserInterface|CreateWidget "/Game/UI/HUD/W_HUD.W_HUD_C" self))
  (bind _output_get (Variables|Default|SetW_HUD_Reference _returnvalue))
  (UserInterface|Viewport|AddtoViewport _output_get 0)
  ;[0.1099 0.4809 1] Obtenemos referencia al GameMode
  (CallFunction|GetGameModeReference)
  ;[0.1099 0.4809 1] Obtenemos referencia al Character del Player
  (CallFunction|GetPlayerCharacterReference)
  ;[0.04519 0.1946 0.4072] Configuramos el Input para que solo reciba Inputs de juego
  (CallFunction|SetIputtoGameMode)
  ;[0.1099 0.4809 1] Agregamos un Contexto de Mapeo de Acciones utilizando el Enhanced Input PlayerSubsystem | Permite controlar el Movimiento del Player
  (Input|AddMappingContext (PlayerController|LocalPlayerSubsystems|GetEnhancedInputLocalPlayerSubsystem self) "/Game/Blueprints/Player/Input/IMC_PlayerMovement.IMC_PlayerMovement" 0 "(bIgnoreAllPressedKeysUntilRelease=True,bForceImmediately=False,bNotifyUserSettings=False)"))

(event EventTick
  (params (DeltaSeconds :type Float%20%28single-precision%29)))

(event Input|ActionEvents|InputActionInteractWithDialogue
  (params (Key :type Key%20Structure :default "None"))
  (:Pressed
    ;[1 0.1136 0.1534] Revisamos si el Player se encuentra en un dialogo
    (if (Variables|/Game/Blueprints/Player/BP_MyCharacter.BP_MyCharacter_C|GetInDialogue (Variables|Default|GetPlayerCharacter))
      ;[0.3012 1 0.6906] Solicitamos que se continúe con el Diálogo
      (Default|AsktoContinueDialogue (Variables|Default|GetGameModeReference))
      (else
        ;[0.3012 1 0.6906] Solicitar inicio de Dialogo, en caso
        ;;[1 1 1] Revisamos si tenemos una referenciaa un NPC cercano
        (bind _nearnpc (Variables|/Game/Blueprints/Player/BP_MyCharacter.BP_MyCharacter_C|GetNearNPC (Variables|Default|GetPlayerCharacter))
          (:then
            ;;[1 1 1] En caso si la tengamos, solicitamos al GameManager que muestre su Dialogo
            (Default|AskforDialogue (Variables|Default|GetGameModeReference) _nearnpc)
            ;[1 0.3104 0.2806] Activamos Flag de Jugador en Dialogo
            (Variables|/Game/Blueprints/Player/BP_MyCharacter.BP_MyCharacter_C|SetInDialogue (Variables|Default|GetPlayerCharacter) true)
            ;[1 0.3104 0.2806] Desactivamos Flag de "Jugador puede moverse"
            (Variables|/Game/Blueprints/Player/BP_MyCharacter.BP_MyCharacter_C|SetCanMove (Variables|Default|GetPlayerCharacter) false))
          (:else))))))

(event Input|ActionEvents|InputActionStart/Pause
  (params (Key :type Key%20Structure :default "None"))
  (:Pressed
    (CallFunction|ChangeLevel "MainMenu")))

(event Input|ActionEvents|InputActionUseSoulLight
  (params (Key :type Key%20Structure :default "None"))
  (:Pressed
    ;[1 0.4626 0] Hacer que el Player utilice la Luz de Alma
    (Default|UseSoulLight (Variables|Default|GetPlayerCharacter))))

(fn ConstructionScript)

(fn GetPlayerCharacterReference
  (bind _asbp_my_character (Utilities|Casting|CastToBP_MyCharacter (Pawn|GetControlledPawn)))
  (Variables|Default|SetPlayerCharacter _asbp_my_character))

(fn GetGameModeReference
  (bind _asbp_ecgame_mode (Utilities|Casting|CastToBP_ECGameMode (Game|GetGameMode)))
  (Variables|Default|SetGameModeReference _asbp_ecgame_mode))

(fn SetIputtoGameMode
  (Input|SetInputModeGameOnly self false)
  (Variables|Default|SetbShowMouseCursor false))