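; Player controller that drives the player character's movement and starts NPC dialogue.
; On BeginPlay it caches the game mode and controlled character, then adds an Enhanced Input mapping context for movement.
; Move input applies only single-axis movement, ignoring diagonals, while the character can move, and stores its direction.
; The interact action asks the game mode for the nearby NPC's dialogue, then flags the character as in dialogue and unable to move.
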(event Input|EnhancedActionEvents|EnhancedInputActionIA_Move
  (params (ActionValue :type Vector%202D%20Structure) (ElapsedSeconds :type Float%20%28double-precision%29) (TriggeredSeconds :type Float%20%28double-precision%29) (InputAction :type Input%20Action%20Object%20Reference :default "/Game/Blueprints/Player/Input/IA_Move.IA_Move"))
  ;[0.06447 0.4112 1] Evento de Inputs de Movimiento
  ;;[0.8438 0.1187 0.1453] Comprobamos si el Personaje puede moverse
  (if (Variables|/Game/Blueprints/Player/BP_MyCharacter.BP_MyCharacter_C|GetCanMove (Variables|Default|GetPlayerCharacter))
    (if (and (!= (.x ActionValue) 0.0) (== (.y ActionValue) 0.0))
      ;;[0.1099 0.4809 1] Agregamos Inputs de movimiento al Perosnaje
      (Pawn|Input|AddMovementInput (Variables|Default|GetPlayerCharacter) (Transformation|GetActorRightVector (Variables|Default|GetPlayerCharacter)) (.x ActionValue) false)
      ;;[1 1 1] Actualizamos la variable de Dirección del Player
      (Variables|/Game/Blueprints/Player/BP_MyCharacter.BP_MyCharacter_C|SetDirection (Variables|Default|GetPlayerCharacter) (Math|Vector2D|MakeVector2D (.x ActionValue) (.y ActionValue)) :!label _label)
      (elif (and (== (.x ActionValue) 0.0) (!= (.y ActionValue) 0.0))
        (Pawn|Input|AddMovementInput (Variables|Default|GetPlayerCharacter) (Transformation|GetActorForwardVector (Variables|Default|GetPlayerCharacter)) (.y ActionValue) false)
        (goto _label)))))

(event EventBeginPlay
  ;[0.1099 0.4809 1] Obtenemos referencia al GameMode
  (CallFunction|GetGameModeReference)
  ;[0.1099 0.4809 1] Obtenemos referencia al Character del Player
  (CallFunction|GetPlayerCharacterReference)
  ;[0.1099 0.4809 1] Agregamos un Contexto de Mapeo de Acciones utilizando el Enhanced Input PlayerSubsystem | Permite controlar el Movimiento del Player
  (Input|AddMappingContext (PlayerController|LocalPlayerSubsystems|GetEnhancedInputLocalPlayerSubsystem self) "/Game/Blueprints/Player/Input/IMC_PlayerMovement.IMC_PlayerMovement" 0 "(bIgnoreAllPressedKeysUntilRelease=True,bForceImmediately=False,bNotifyUserSettings=False)"))

(event EventTick
  (params (DeltaSeconds :type Float%20%28single-precision%29)))

(event Input|ActionEvents|InputActionInteractWithDialogue
  (params (Key :type Key%20Structure :default "None"))
  (:Pressed
    ;[1 0.1136 0.1534] Revisamos que el Player no se encuentre en un dialogo
    (if (not (Variables|/Game/Blueprints/Player/BP_MyCharacter.BP_MyCharacter_C|GetInDialogue (Variables|Default|GetPlayerCharacter)))
      ;[0.3012 1 0.6906] Solicitar inicio de Dialogo, en caso
      ;;[1 1 1] Revisamos si tenemos una referenciaa un NPC cercano
      (bind _nearnpc (Variables|/Game/Blueprints/Player/BP_MyCharacter.BP_MyCharacter_C|GetNearNPC (Variables|Default|GetPlayerCharacter))
        (:then
          ;;[1 1 1] En caso si la tengamos, solicitamos al GameManager que muestre su Dialogo
          (Default|AskforDialogue (Variables|Default|GetGameModeReference) _nearnpc)
          ;[1 1 1] Activamos Flag de Jugador en Dialogo
          (Variables|/Game/Blueprints/Player/BP_MyCharacter.BP_MyCharacter_C|SetInDialogue (Variables|Default|GetPlayerCharacter) true)
          ;[1 1 1] Desactivamos Flag de "Jugador puede moverse"
          (Variables|/Game/Blueprints/Player/BP_MyCharacter.BP_MyCharacter_C|SetCanMove (Variables|Default|GetPlayerCharacter) false))
        (:else)))))

(fn ConstructionScript)

(fn GetPlayerCharacterReference
  (bind _asbp_my_character (Utilities|Casting|CastToBP_MyCharacter (Pawn|GetControlledPawn)))
  (Variables|Default|SetPlayerCharacter _asbp_my_character))

(fn GetGameModeReference
  (bind _asbp_ecgame_mode (Utilities|Casting|CastToBP_ECGameMode (Game|GetGameMode)))
  (Variables|Default|SetGameModeReference _asbp_ecgame_mode))