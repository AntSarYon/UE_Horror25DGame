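; Player character that carries a Soul Light, which it can drop in place or recall.
; A dropped light is pinned to its saved location on Tick; recall lerps it back on a timeline, with stun mode active during the return.
; It also tracks a nearby interactable and its widget, updates a movement flag for animation, and plays a one-time sound on hitting a guardian enemy.
; Events reparent the camera to a given component or back to the spring arm.
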(event OnComponentBeginOverlap(InteractionDetectionArea)
  (params (OverlappedComponent :type Primitive%20Component%20Object%20Reference) (OtherActor :type Actor%20Object%20Reference) (OtherComp :type Primitive%20Component%20Object%20Reference) (OtherBodyIndex :type Integer) (bFromSweep :type Boolean) (SweepResult :type Hit%20Result%20Structure%20%28by%20ref%29))
  ;[0.6476 0.5 1] INTERACCIÓN CON NPCs
  ;;[0.6983 0.4166 1] En caso el Actor detectado sea un NPC, almsecnamos su referencia
  (bind _asbp_interactable_actor (Utilities|Casting|CastToBP_InteractableActor OtherActor))
  (bind _output_get (Variables|DialogueInteractions|SetNearNPC _asbp_interactable_actor))
  (Default|ShowInteractionWidget _output_get))

(event OnComponentEndOverlap(InteractionDetectionArea)
  (params (OverlappedComponent :type Primitive%20Component%20Object%20Reference) (OtherActor :type Actor%20Object%20Reference) (OtherComp :type Primitive%20Component%20Object%20Reference) (OtherBodyIndex :type Integer))
  (bind _interactiondetectionarea (Variables|Default|GetInteractionDetectionArea))
  (bind _overlappingactors (Collision|GetOverlappingActors _interactiondetectionarea "/Game/Blueprints/Interactables/BP_InteractableActor.BP_InteractableActor_C" :!class /Script/Engine.PrimitiveComponent))
  (bind _returnvalue (Utilities|Array|Length _overlappingactors))
  ;[0.6476 0.5 1] INTERACCIÓN CON NPCs
  ;;[0.5876 0.3953 1] En caso el Actor sea un NPC, desactivamos su widget, a la vez que quitamos su referencia (si le correspondía)
  (bind _asbp_interactable_actor (Utilities|Casting|CastToBP_InteractableActor OtherActor))
  (Default|HideInteractionWidget _asbp_interactable_actor)
  (if (== _asbp_interactable_actor (Variables|DialogueInteractions|GetNearNPC))
    (Variables|DialogueInteractions|SetNearNPC 0)
    ;;[0.2384 0.162 0.4072] Revisamos si hay algun otro Actor que esté Solapando, y en caso lo haya, lo seteamos como el Nuevo NPC Cercano
    (if (>= _returnvalue 1)
      (bind _asbp_interactable_actor_2 (Utilities|Casting|CastToBP_InteractableActor (Utilities|Array|Get(acopy) _overlappingactors (- _returnvalue 1))))
      (Variables|DialogueInteractions|SetNearNPC _asbp_interactable_actor_2))))

(event OnComponentHit(CapsuleComponent)
  (params (HitComponent :type Primitive%20Component%20Object%20Reference) (OtherActor :type Actor%20Object%20Reference) (OtherComp :type Primitive%20Component%20Object%20Reference) (NormalImpulse :type Vector :default "0, 0, 0") (Hit :type Hit%20Result%20Structure%20%28by%20ref%29))
  (Utilities|Casting|CastToBP_EnemieGuardian OtherActor)
  (Utilities|FlowControl|DoOnce false
    (:Completed
      (Audio|PlaySound2D "/Game/Audio/Screamer/Kya_Cue.Kya_Cue" 1.0 1.0 0.0 0 0))))

(event Custom|RecoverLightSoul
  ;[1 0.4626 0] Interactuar con la Luz de Alma
  ;;[1 0.912 0.4225] Reproducimos sonido de Luz
  (Audio|PlaySoundatLocation "/Game/Audio/SoulLight/SC_ReturningLight.SC_ReturningLight" (Variables|SoulLight|GetSoulLightLastLocation) "0, 0, 0" 1.0 1.0 0.0 "/Game/Audio/SoulLight/SA_ReturningLight.SA_ReturningLight" 0 0 0)
  ;;[0.1384 0.003677 0.001518] Activamos el Stun de la Luz
  (Default|EnableStunMode (Variables|SoulLight|GetSoulLight))
  ;;[1 0.81 0.2118] Llevamos la Luz de vuelta a la posición del Player
  ;;;[1 1 1] Interpolamos la ubicacion de la Luz
  (bind _lightlocationinterpolation (Timeline|SoluLightComeBack PlayFromStart)
    (:Update
      (Transformation|SetActorLocation (Variables|SoulLight|GetSoulLight) (Math|Vector|Lerp(Vector) (Variables|SoulLight|GetSoulLightLastLocation) (Transformation|GetActorLocation) _lightlocationinterpolation) true false))
    (:Finished
      ;;;[0.1384 0.003677 0.001518] Desactivamos el Stun de la Luz
      (Default|DisableStunMode (Variables|SoulLight|GetSoulLight)))))

(event Custom|RestoreCamera
  ;[0.03955 0.09306 0.1413] Hacemos que la cámara vuelva a su posición original
  (Transformation|AttachComponentToComponent (Variables|Default|GetCamera) (Variables|Default|GetSpringArm) "None" "KeepRelative" "KeepRelative" "KeepRelative" true))

(event Custom|UseSoulLight
  ;[1 0.4626 0] Interactuar con la Luz de Alma
  ;;[1 0.125 0.125] Revisamos si la Luz esta, o no, Atada a nosotros
  (if (Variables|/Game/Blueprints/Player/SoulLight/BP_SoulLight.BP_SoulLight_C|GetIsAttached (Variables|SoulLight|GetSoulLight))
    ;;[1 0.81 0.2118] Guardamos la ultima ubicacion de la Luz
    (SoulLight|SaveSoulLightLastLocation)
    ;;[1 0.81 0.2118] Desactivamos el Flag de Luz Atada
    (Variables|/Game/Blueprints/Player/SoulLight/BP_SoulLight.BP_SoulLight_C|SetIsAttached (Variables|SoulLight|GetSoulLight) false)
    (else
      ;;[1 0.81 0.2118] Activamos el Flag de Luz Atada y e invocamops al Evento de Recuperar Luz | y
      (Variables|/Game/Blueprints/Player/SoulLight/BP_SoulLight.BP_SoulLight_C|SetIsAttached (Variables|SoulLight|GetSoulLight) true)
      (CallFunction|RecoverLightSoul))))

(event Custom|MoveCameraToGate
  (params (NewParentComponent :type Scene%20Component%20Object%20Reference))
  ;[0.02956 0.07227 0.107] Movemos la Camara hacia una nueva posicion
  (Transformation|AttachComponentToComponent (Variables|Default|GetCamera) NewParentComponent "None" "KeepRelative" "KeepRelative" "KeepRelative" true))

(event EventBeginPlay
  ;[1 0.4626 0] Obtenemos la Referencia a la Luz del Alma
  (SoulLight|GetSoulLightReference))

(event EventTick
  (params (DeltaSeconds :type Float%20%28single-precision%29))
  ;[0.07997 0.08963 1] Revisamos constantemente si el perosnaje se está moviendo | CRUCIAL PARA ANIMACIONES
  (Movement|CheckifMoving)
  ;[1 0.4626 0] Mantener la última posición de la Luz si no está atada a nosotros.
  (if (not (Variables|/Game/Blueprints/Player/SoulLight/BP_SoulLight.BP_SoulLight_C|GetIsAttached (Variables|SoulLight|GetSoulLight)))
    (Transformation|SetActorLocation (Variables|SoulLight|GetSoulLight) (Variables|SoulLight|GetSoulLightLastLocation) true false)))

(fn ConstructionScript)

(fn CheckifMoving
  (Variables|Movement|SetIsMoving (> (Math|Vector|VectorLength (Variables|/Script/Engine.MovementComponent|GetVelocity (Variables|Character|GetCharacterMovement))) 0.0)))

(fn GetSoulLightReference
  (bind _asbp_soul_light (Utilities|Casting|CastToBP_SoulLight (Variables|/Script/Engine.ChildActorComponent|GetChildActor (Variables|Default|GetSoulLight_ActorComponent))))
  (Variables|SoulLight|SetSoulLight _asbp_soul_light))

(fn SaveSoulLightLastLocation
  (Variables|SoulLight|SetSoulLightLastLocation (Transformation|GetActorLocation (Variables|SoulLight|GetSoulLight))))