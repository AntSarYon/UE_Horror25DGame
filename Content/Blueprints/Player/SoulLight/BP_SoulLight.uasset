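; BP_SoulLight is a light actor that gradually fades while the player character is moving.
; On BeginPlay it caches references to BP_MyCharacter and its BP_MyPlayerController.
; Each Tick, if the character's IsMoving is true, it reduces the point light's intensity, source radius and attenuation radius, and the spot light's intensity and cone angles, scaled by delta time.
; No clamping or restoring of the light happens here.
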(event EventBeginPlay
  ;[1 1 1] Obtenemos referencia al Personaje del Jugador
  (CallFunction|GetPlayerReference))

(event Collision|EventActorBeginOverlap
  (params (OtherActor :type Actor%20Object%20Reference)))

(event EventTick
  (params (DeltaSeconds :type Float%20%28single-precision%29))
  (bind _pointlightdecreasespeed (Variables|LightIntensity|GetPointLightDecreaseSpeed))
  (bind _returnvalue (* _pointlightdecreasespeed DeltaSeconds))
  ;[1 0.1141 0.1041] Revisamos si el Jugador se esta Moviendo
  (if (Variables|/Game/Blueprints/Player/BP_MyCharacter.BP_MyCharacter_C|GetIsMoving (Variables|References|GetPlayerReference))
    ;[1 1 1] Actualizamos la Intensidad de Luz de las Luces
    (Utilities|FlowControl|Sequence
      (:then_0
        (Rendering|Components|Light|SetIntensity (Variables|Default|GetPointLight) (- (Variables|/Script/Engine.LightComponentBase|GetIntensity (Variables|Default|GetPointLight)) _returnvalue))
        (Class|PointLightComponent|SetSourceRadius (Variables|Default|GetPointLight) (- (Variables|/Script/Engine.PointLightComponent|GetSourceRadius (Variables|Default|GetPointLight)) _returnvalue))
        (Rendering|Lighting|SetAttenuationRadius (Variables|Default|GetPointLight) (- (Variables|/Script/Engine.LocalLightComponent|GetAttenuationRadius (Variables|Default|GetPointLight)) (* (+ (Variables|LightIntensity|GetPointLightDecreaseSpeed) 1.0) DeltaSeconds))))
      (:then_1
        (Rendering|Components|Light|SetIntensity (Variables|Default|GetSpotLight) (- (Variables|/Script/Engine.LightComponentBase|GetIntensity (Variables|Default|GetSpotLight)) (* DeltaSeconds (Variables|LightIntensity|GetSpotLightDecreaseSpeed))))
        (Rendering|Lighting|SetInnerConeAngle (Variables|Default|GetSpotLight) (- (Variables|/Script/Engine.SpotLightComponent|GetInnerConeAngle (Variables|Default|GetSpotLight)) (* DeltaSeconds 0.1)))
        (Rendering|Lighting|SetOuterConeAngle (Variables|Default|GetSpotLight) (- (Variables|/Script/Engine.SpotLightComponent|GetOuterConeAngle (Variables|Default|GetSpotLight)) (* DeltaSeconds 0.14)))))))

(fn ConstructionScript)

(fn GetPlayerReference
  ;[1 1 1] Obtenemos referencia al BP del Player
  (bind _asbp_my_character (Utilities|Casting|CastToBP_MyCharacter (Game|GetPlayerCharacter 0)))
  (bind _output_get (Variables|References|SetPlayerReference _asbp_my_character))
  ;[1 1 1] Obtenemos referencia la Player Controller
  (bind _asbp_my_player_controller (Utilities|Casting|CastToBP_MyPlayerController (Pawn|GetController _output_get)))
  (Variables|References|SetPlayerControllerReference _asbp_my_player_controller))