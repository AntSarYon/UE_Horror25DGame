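; Interactable actor, such as an NPC, that loads its dialogue lines and shows or hides an interaction prompt widget.
; On BeginPlay it reads its first row from DT_InteractionsTable_Escenario1, whose text box count sets the multiple-dialogue flag and drives GetDialogueRows to append remaining lines to Dialogues.
; Row names are built by convention from a five-character interaction type prefix, the actor's Name variable, the line index and the current level name.
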(event Custom|ShowInteractionWidget
  (Rendering|SetVisibility (Variables|Default|GetWidget) true false))

(event Custom|HideInteractionWidget
  (Rendering|SetVisibility (Variables|Default|GetWidget) false false))

(event EventBeginPlay
  ;[0 0 0] Obtenemos el Nombre que deberia tener la Fila del DatTable destinada a este NPC
  (bind _rowname (CallFunction|GetDialogueRowName 1))
  ;[0 0 0] Buscamos la Fila en el DataTable de Dialogos
  (bind _returnvalue (Utilities|GetDataTableRow "/Game/DataStructures/DT_InteractionsTable_Escenario1.DT_InteractionsTable_Escenario1" _rowname)
    (:then
      ;[1 0.07268 0.09258] Revisamos si el numero de Dialogos es mayor a 1
      (bind _output_get (Variables|Default|SetNumberOfDialogues (.NumberOfTextBoxes (Utilities|Struct|BreakES_InteractionData _returnvalue))))
      (if (> _output_get 1)
        ;[1 0.1041 0.1141] Activamos el Flag de Multiples dialogos
        (Variables|Default|SetHasMultipleDialogues true)
        ;[1 0.399 0.6562] Almacenamos el único Dialogo en el Array de Dialogos
        (Variables|NPC_Data|SetDialogues (Utilities|Array|MakeArray (.DialogueText (Utilities|Struct|BreakES_InteractionData _returnvalue))))
        (CallFunction|GetDialogueRows)
        (else
          ;[1 0.1041 0.1141] Desactivamos el Flag de multiples dialogos
          (Variables|Default|SetHasMultipleDialogues false)
          ;[1 0.399 0.6562] Almacenamos el único Dialogo en el Array de Dialogos
          (Variables|NPC_Data|SetDialogues (Utilities|Array|MakeArray (.DialogueText (Utilities|Struct|BreakES_InteractionData _returnvalue)))))))
    (:RowNotFound
      (Development|PrintString "No encontré ningun Dialogo para este NPC"))))

(event Collision|EventActorBeginOverlap
  (params (OtherActor :type Actor%20Object%20Reference)))

(event EventTick
  (params (DeltaSeconds :type Float%20%28single-precision%29)))

(fn ConstructionScript)

(fn GetDialogueRowName
  (params (Indice :type Integer))
  (bind _returnvalue (Game|GetCurrentLevelName true))
  (return (Utilities|String|StringToName (Utilities|String|Append (Utilities|String|Left (Utilities|String|EnumtoString (Variables|NPC_Data|GetInteractionType)) 5) (Variables|NPC_Data|GetName) (Utilities|String|ToString(Integer) Indice) _returnvalue))))

(fn GetDialogueRows
  ;[0.2634 1 0.6472] Por cada Fila que debe encontrarse en el DatTable
  (for _index (range 2 (Variables|Default|GetNumberOfDialogues))
    (bind _rowname (CallFunction|GetDialogueRowName _index))
    (bind _returnvalue (Utilities|GetDataTableRow "/Game/DataStructures/DT_InteractionsTable_Escenario1.DT_InteractionsTable_Escenario1" _rowname)
      (:then
        (Utilities|Array|Add (Variables|NPC_Data|GetDialogues) (.DialogueText (Utilities|Struct|BreakES_InteractionData _returnvalue)))))))