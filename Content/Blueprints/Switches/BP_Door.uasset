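; BP_Door is a door actor that opens once all of its registered switches are activated.
; On BeginPlay it stores closed and offset open positions, then binds to each switch's OnSwitchActivated event.
; Each activation scans the switch array and calls Open if none is inactive.
; Open runs through a DoOnce, playing a sound and a Timeline that lerps the door mesh sideways to its final position.
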(event Custom|Open
  (Utilities|FlowControl|DoOnce false
    (:Completed
      ;[0.08022 0.1845 0.2789] Reproducimos Sonido de Puerta abriendose
      (Audio|PlaySoundatLocation "/Game/Audio/Door/BigDoorOpen_Cue.BigDoorOpen_Cue" (Transformation|GetWorldLocation (Variables|Default|GetDoorMesh)) "0, 0, 0" 1.0 1.0 0.0 0 0 0 0)
      ;[0.107 0.06848 0.009134] Reproducimos TimeLine para controlar la Interpolacion de Posicion de la Puerta
      (bind _interpolation (Timeline|Timeline Play)
        (:Update
          (Transformation|SetRelativeLocation (Variables|Default|GetDoorMesh) (Math|Vector|Lerp(Vector) (Variables|Default|GetInitialLocation) (Variables|Default|GetFinalLocation) _interpolation) false false))))))

(event Custom|CheckSwitches
  (CallFunction|CheckifAllSwitchesAreActivate))

(event EventBeginPlay
  ;[0.9647 0.5711 0.01681] Obtenemos la Ubicacion original de la Puerta
  (bind _output_get (Variables|Default|SetInitialLocation (Variables|/Script/Engine.SceneComponent|GetRelativeLocation (Variables|Default|GetDoorMesh))))
  ;[0.9823 0.5841 0.01681] Asignamos la Ubicacion Final de la Puerta
  (Variables|Default|SetFinalLocation (+ _output_get "0.000000,-450.000000,0.000000"))
  ;[0 0.402 0.9131] Por cada Switch registrado
  (for _array_element (Variables|Default|GetArrSwitches)
    ;[0.05127 0.1248 0.1878] Vamos a Asignar un Evento Delegados a la Activación de cada Switch
    (EventDispatchers|BindEventtoOnSwitchActivated _array_element (delegate Custom|CheckSwitches))))

(event Collision|EventActorBeginOverlap
  (params (OtherActor :type Actor%20Object%20Reference)))

(event EventTick
  (params (DeltaSeconds :type Float%20%28single-precision%29)))

(fn ConstructionScript)

(fn CheckifAllSwitchesAreActivate
  ;[0.0999 0.0999 0.0999] Por cada Switch en el Array
  (bind _array_element (Utilities|Array|ForEachLoopwithBreak (Variables|Default|GetArrSwitches) :!label _label)
    (:LoopBody
      ;;[0.2961 0 0] Revisamos si esta activado
      (if (not (Variables|/Game/Blueprints/Switches/BP_Switch.BP_Switch_C|GetIsActivated _array_element))
        ;;[0.2918 0 0] Si no esta activo, desactivamos el Flag de TTodos Activados e interrumpimos el Bucle
        (LocalVariables|SetAllActivated false)
        (goto _label Break)))
    (:Completed
      ;;[0.2961 0 0] Si todos los Switches, en efecto, estan activos
      (if (LocalVariables|GetAllActivated)
        ;;[0.05613 0.1195 0.1779] Llamamos al Evento de Abrir la Puerta
        (CallFunction|Open)))))