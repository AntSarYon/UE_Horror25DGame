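; BP_Switch is a one-shot pressure switch that enemy guardians can always trigger, and the player only when CanBeActivatedByPlayer is set.
; On BeginPlay that flag selects the player or enemy material for the switch mesh.
; Trigger overlaps count only for capsule components of a valid actor.
; The first valid overlap lowers the mesh, applies the activated material, sets IsActivated and fires the SwitchActivated dispatcher.
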(event OnComponentBeginOverlap(SwitchTrigger)
  (params (OverlappedComponent :type Primitive%20Component%20Object%20Reference) (OtherActor :type Actor%20Object%20Reference) (OtherComp :type Primitive%20Component%20Object%20Reference) (OtherBodyIndex :type Integer) (bFromSweep :type Boolean) (SweepResult :type Hit%20Result%20Structure%20%28by%20ref%29))
  ;[0.005182 0.1144 0.1221] Casteamos el otro Actor como el Enemgo
  (Utilities|Casting|CastToCapsuleComponent OtherComp)
  (Utilities|Casting|CastToBP_EnemieGuardian OtherActor
    (:then
      (Utilities|FlowControl|DoOnce false :!label _label
        (:Completed
          ;[0.07421 0.1878 0.3005] Chancamos el Switch en el Suelo
          (Transformation|AddWorldOffset (Variables|Default|GetSwitchMesh) "0.000000,0.000000,-20.000000" false false)
          ;[0.03955 0.1022 0.162] Modificamos el Material del Switch
          (Rendering|Material|SetMaterial (Variables|Default|GetSwitchMesh) 0 (Variables|Default|GetMatActivatedSwitch))
          ;[0.1559 0.001821 0.001518] Activamos el Flag de "Esta Activado"
          (Variables|ActivationFlags|SetIsActivated true)
          ;[0.03955 0.09531 0.147] Llamamos a los Delegados del Evento "SwitchActivated"
          (Default|CallOnSwitchActivated))))
    (:CastFailed
      ;[0.2961 0 0] En caso no sea enemigo, revisamos si el Flag de "Activado por jugador" esta activo
      (if (Variables|ActivationFlags|GetCanBeActivatedByPlayer)
        ;[0.02732 0.1441 0.15] Volvemos a hacer un Casteo del Actor, pero esta vez como el Player
        (Utilities|Casting|CastToBP_MyCharacter OtherActor)
        (goto _label)))))

(event EventBeginPlay
  (if (Variables|ActivationFlags|GetCanBeActivatedByPlayer)
    (Rendering|Material|SetMaterial (Variables|Default|GetSwitchMesh) 0 (Variables|Default|GetMatPlayerSwitch))
    (else
      (Rendering|Material|SetMaterial (Variables|Default|GetSwitchMesh) 0 (Variables|Default|GetMatEnemieSwitch)))))

(event Collision|EventActorBeginOverlap
  (params (OtherActor :type Actor%20Object%20Reference)))

(event EventTick
  (params (DeltaSeconds :type Float%20%28single-precision%29)))

(fn ConstructionScript)