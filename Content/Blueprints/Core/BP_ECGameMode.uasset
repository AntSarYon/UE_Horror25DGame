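; BP_ECGameMode is a game mode that relays NPC dialogue requests to the level's BP_DialogueManager.
; On BeginPlay it caches the dialogue manager, found by actor class, and the first player's BP_MyPlayerController.
; AskForDialogue passes the NPC's name, dialogues, talk speed and interaction type to the manager to display.
; AskToContinueDialogue forwards the continue request to the manager; the cached controller is not used here.
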(event Custom|AskForDialogue
  (params (NPCCharacter :type BP%20Interactable%20Actor%20Object%20Reference))
  ;[0.7378 0.4158 1] Enviamos al DialogueManager la informacion de Dialogo que contiene el NPC recibido
  (Default|ShowDialogues (Variables|Managers|GetDialogueManager) (Variables|/Game/Blueprints/Interactables/BP_InteractableActor.BP_InteractableActor_C|GetName NPCCharacter) (Variables|/Game/Blueprints/Interactables/BP_InteractableActor.BP_InteractableActor_C|GetDialogues NPCCharacter) (Variables|/Game/Blueprints/Interactables/BP_InteractableActor.BP_InteractableActor_C|GetTalkSpeed NPCCharacter) (Variables|/Game/Blueprints/Interactables/BP_InteractableActor.BP_InteractableActor_C|GetInteractionType NPCCharacter)))

(event Custom|AskToContinueDialogue
  ;[0.4072 0 0.08438] Le ordenamos al DialogueManager que continúe con el diálogo, o cierre el panel
  (Default|ContinueDialogue (Variables|Managers|GetDialogueManager)))

(event EventBeginPlay
  ;[0 0 0] Obtenemos Referencia al DialogueManager
  (CallFunction|GetDialogueManager)
  ;[0 0 0] Obtenemos referencia al Player Controller
  (CallFunction|GetPlayerController))

(fn ConstructionScript)

(fn GetDialogueManager
  (bind _returnvalue (Actor|GetActorOfClass "/Game/Blueprints/Managers/BP_DialogueManager.BP_DialogueManager_C"))
  (Variables|Managers|SetDialogueManager _returnvalue))

(fn GetPlayerController
  (bind _asbp_my_player_controller (Utilities|Casting|CastToBP_MyPlayerController (Game|GetPlayerController 0)))
  (Variables|Player|SetPlayerControllerReference _asbp_my_player_controller))